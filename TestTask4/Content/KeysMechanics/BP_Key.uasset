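; BP_Key is a key actor that the third-person character can pick up, drop or set into a place.
; Overlap triggers register it as the character's ActorToPickUp and show a text render turned to the follow camera on entry.
; SetKeyPlaced flags it as placed or handled, then a Timeline glides it toward the target and disables collision and physics.
; DropKey detaches it and restores physics, gravity and collision.
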(event `self.ReceiveBeginPlay`
  (`SceneComponent.SetVisibility` (`self.TextRender`) false false))

(event `SetKeyPlaced`
  (params (NewPlace :type "Vector Structure") (SetPlaced :type Boolean))
  (bind _keymesh (`self.KeyMesh`))
  (bind _returnvalue (`self.K2_GetActorLocation` self))
  (`SceneComponent.SetVisibility` (`self.TextRender`) false false)
  (if SetPlaced
    (set `self.bIsPlaced` true)
    (bind (_direction _newtrack_0) (`Timeline|Timeline` :!label _label)
      (:`Update`
        (`self.K2_SetActorLocation` self (+ _returnvalue (* (`KismetMathLibrary.GetForwardVector` (`KismetMathLibrary.FindLookAtRotation` _returnvalue NewPlace)) (* (`KismetMathLibrary.Vector_Distance` _returnvalue NewPlace) _newtrack_0))) false false))
      (:`Finished`
        (`self.SetActorEnableCollision` self false)
        (`PrimitiveComponent.SetSimulatePhysics` _keymesh false)
        (`PrimitiveComponent.SetCollisionEnabled` _keymesh "NoCollision")))
    (else
      (set `self.bIsHandled` true)
      (goto _label))))

(event `self.PickUpTrigger.OnComponentBeginOverlap`
  (params (OverlappedComponent :type "PrimitiveComponent Object Reference") (OtherActor :type "Actor Object Reference") (OtherComp :type "PrimitiveComponent Object Reference") (OtherBodyIndex :type Integer) (bFromSweep :type Boolean) (SweepResult :type "HitResult Structure (by ref)"))
  (if (not (`self.bIsPlaced`))
    (bind _asbp_third_person_character (cast `/Game/ThirdPerson/Blueprints/BP_ThirdPersonCharacter` OtherActor))
    (set `/Game/ThirdPerson/Blueprints/BP_ThirdPersonCharacter.ActorToPickUp` self _asbp_third_person_character)))

(event `DropKey`
  (bind _keymesh (`self.KeyMesh`))
  (`self.K2_DetachFromActor` "KeepWorld" "KeepWorld" "KeepWorld")
  (`PrimitiveComponent.SetCollisionEnabled` _keymesh "QueryAndPhysics")
  (`PrimitiveComponent.SetSimulatePhysics` _keymesh true)
  (`PrimitiveComponent.SetEnableGravity` _keymesh true)
  (set `self.bIsHandled` false)
  (`self.SetActorEnableCollision` self true))

(event `self.TextTrigger.OnComponentBeginOverlap`
  (params (OverlappedComponent :type "PrimitiveComponent Object Reference") (OtherActor :type "Actor Object Reference") (OtherComp :type "PrimitiveComponent Object Reference") (OtherBodyIndex :type Integer) (bFromSweep :type Boolean) (SweepResult :type "HitResult Structure (by ref)"))
  (bind _textrender (`self.TextRender`))
  ;[1 1 1] Show text render
  (if (`self.bIsPlaced`)
    _
    (elif (not (`self.bIsHandled`))
      (bind _asbp_third_person_character (cast `/Game/ThirdPerson/Blueprints/BP_ThirdPersonCharacter` OtherActor))
      (`SceneComponent.K2_SetWorldRotation` _textrender (`KismetMathLibrary.FindLookAtRotation` (`SceneComponent.K2_GetComponentLocation` _textrender) (`SceneComponent.K2_GetComponentLocation` (`/Game/ThirdPerson/Blueprints/BP_ThirdPersonCharacter.FollowCamera` _asbp_third_person_character))) false false)
      (`SceneComponent.SetVisibility` _textrender true false))))

(event `self.TextTrigger.OnComponentEndOverlap`
  (params (OverlappedComponent :type "PrimitiveComponent Object Reference") (OtherActor :type "Actor Object Reference") (OtherComp :type "PrimitiveComponent Object Reference") (OtherBodyIndex :type Integer))
  ;[1 1 1] Show text render
  (`SceneComponent.SetVisibility` (`self.TextRender`) false false))

(fn `UserConstructionScript`)