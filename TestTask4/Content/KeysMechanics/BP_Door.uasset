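; BP_Door is a two-key door that slides open after receiving a second unlock call from a BP_KeyStand.
; The first call only sets a flag; the next plays a Timeline that adds a scaled Z offset to the door's current position each update.
; A trigger reveals a TextRender, turned once toward the player's camera on overlap, while Closed is true; opening also sets Closed true.
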(event `self.ReceiveBeginPlay`
  (`SceneComponent.SetVisibility` (`self.TextRender`) false false))

(event `OpenDoor`
  (bind _door (`self.Door`))
  ;[1 1 1] Doo opening
  (bind (_direction _offset) (`Timeline|Timeline`)
    (:`Update`
      (`SceneComponent.K2_SetRelativeTransform` _door (`KismetMathLibrary.MakeTransform` (+ (.location (`SceneComponent.GetRelativeTransform` _door)) (`KismetMathLibrary.MakeVector` 0.0 0.0 (* _offset (`self.SlideValue`)))) (.rotation (`SceneComponent.GetRelativeTransform` _door)) (.scale (`SceneComponent.GetRelativeTransform` _door))) false false)
      (set `self.bClosed` true))))

(event `self.TextTrigger.OnComponentBeginOverlap`
  (params (OverlappedComponent :type "PrimitiveComponent Object Reference") (OtherActor :type "Actor Object Reference") (OtherComp :type "PrimitiveComponent Object Reference") (OtherBodyIndex :type Integer) (bFromSweep :type Boolean) (SweepResult :type "HitResult Structure (by ref)"))
  (bind _textrender (`self.TextRender`))
  ;[1 1 1] Show text render
  (if (`self.bClosed`)
    (bind _asbp_third_person_character (cast `/Game/ThirdPerson/Blueprints/BP_ThirdPersonCharacter` OtherActor))
    (`SceneComponent.K2_SetWorldRotation` _textrender (`KismetMathLibrary.FindLookAtRotation` (`SceneComponent.K2_GetComponentLocation` _textrender) (`SceneComponent.K2_GetComponentLocation` (`/Game/ThirdPerson/Blueprints/BP_ThirdPersonCharacter.FollowCamera` _asbp_third_person_character))) false false)
    (`SceneComponent.SetVisibility` _textrender true false)))

(event `self.TextTrigger.OnComponentEndOverlap`
  (params (OverlappedComponent :type "PrimitiveComponent Object Reference") (OtherActor :type "Actor Object Reference") (OtherComp :type "PrimitiveComponent Object Reference") (OtherBodyIndex :type Integer))
  ;[1 1 1] Show text render
  (`SceneComponent.SetVisibility` (`self.TextRender`) false false))

(event `UnlockDoor`
  (params (Instigator :type "Actor Object Reference"))
  ;[1 1 1] Check if instigator is a key stand, opens door if one stand was already set up
  (cast `/Game/KeysMechanics/BP_KeyStand` Instigator)
  (if (`self.bOneKeyIsSet`)
    (`self.OpenDoor`)
    (else
      (set `self.bOneKeyIsSet` true))))

(fn `UserConstructionScript`)